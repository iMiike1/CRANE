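; Background object actor for the runner map that randomizes its look among three placeholder components on BeginPlay.
; A chain of separate random rolls toggles the visibility of at most one placeholder, then the actor destroys itself after a fixed delay.
; Because each check rerolls, the odds are uneven, and when all checks fail nothing toggles and the actor is never destroyed by this graph.
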(event EventBeginPlay
  (bind _returnvalue (Math|Random|RandomIntegerinRange 0 2))
  (if (== _returnvalue 0)
    (Rendering|ToggleVisibility (Variables|Default|GetPlaceHolder1) false)
    (Utilities|FlowControl|Delay 5e+01 :!label _label)
    (Actor|DestroyActor)
    (elif (== _returnvalue 1)
      (Rendering|ToggleVisibility (Variables|Default|GetPlaceHolder2) false)
      (goto _label)
      (elif (== _returnvalue 2)
        (Rendering|ToggleVisibility (Variables|Default|GetPlaceHolder3) false)
        (goto _label)))))

(fn ConstructionScript)