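; A timed 2x score multiplier pickup actor for the runner game.
; When the ThirdPersonCharacter overlaps its box, it sets the game mode's PointsMultiplier to 2, hides the cube, then resets the multiplier to 1 after ten seconds.
; It destroys itself 20 seconds after BeginPlay regardless of pickup, so a late pickup can be destroyed before the reset runs.
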(event OnComponentBeginOverlap(Box)
  (params (OverlappedComponent :type Primitive%20Component%20Object%20Reference) (OtherActor :type Actor%20Object%20Reference) (OtherComp :type Primitive%20Component%20Object%20Reference) (OtherBodyIndex :type Integer) (bFromSweep :type Boolean) (SweepResult :type Hit%20Result%20Structure%20%28by%20ref%29))
  ;[1 1 1] Multiplier Setup
  (Utilities|Casting|CastToThirdPersonCharacter OtherActor)
  (bind _asthird_person_game_mode (Utilities|Casting|CastToThirdPersonGameMode (Game|GetGameMode)))
  (Variables|/Game/ThirdPersonBP/Blueprints/ThirdPersonGameMode.ThirdPersonGameMode_C|SetPointsMultiplier _asthird_person_game_mode 2)
  (Rendering|SetVisibility (Variables|Default|GetCube) false false)
  (Utilities|FlowControl|Delay 1e+01)
  (Variables|/Game/ThirdPersonBP/Blueprints/ThirdPersonGameMode.ThirdPersonGameMode_C|SetPointsMultiplier _asthird_person_game_mode 1))

(event EventBeginPlay
  ;[1 1 1] Destroys non-picked up multiplier
  (Utilities|FlowControl|Delay 2e+01)
  (Actor|DestroyActor))

(event Collision|EventActorBeginOverlap
  (params (OtherActor :type Actor%20Object%20Reference)))

(event EventTick
  (params (DeltaSeconds :type Float%20%28single-precision%29)))

(fn ConstructionScript)