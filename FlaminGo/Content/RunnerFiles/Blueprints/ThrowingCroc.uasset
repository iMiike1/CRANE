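; ThrowingCroc is a crocodile hazard actor that periodically throws bombs, then despawns.
; On BeginPlay it waits briefly, then loops on a fixed delay, spawning a Bomb at its own transform each pass.
; A counter increments after each spawn and the actor destroys itself once it exceeds 30, so it spawns 31 bombs in total.
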(event EventBeginPlay
  ;[1 1 1] Once Spawned Croc throws 30 bombs then despawns
  (Utilities|FlowControl|Delay 1.3)
  (Game|SpawnActorfromClass "/Game/RunnerFiles/Blueprints/Bomb.Bomb_C" (Transformation|GetActorTransform) "Undefined" 0 0 :!label _label)
  (Variables|Default|SetBombsThrown (+ (Variables|Default|GetBombsThrown) 1))
  (if (> (Variables|Default|GetBombsThrown) 30)
    (Actor|DestroyActor)
    (else
      (Utilities|FlowControl|Delay 2.67)
      (goto _label))))

(event Collision|EventActorBeginOverlap
  (params (OtherActor :type Actor%20Object%20Reference))
  ;[1 1 1] Once Spawned Croc throws 30 bombs then despawns
)

(event EventTick
  (params (DeltaSeconds :type Float%20%28single-precision%29)))

(fn ConstructionScript)