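; Desert ground tile for an endless runner that decorates its sides and extends the track as the player moves along.
; On BeginPlay it spawns one MapBackgroundObjects actor at each side spawn point, with a randomized Y offset.
; When the ThirdPersonCharacter overlaps its box, it calls SpawnGround twice on the game mode, then destroys itself after a short delay.
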(event OnComponentBeginOverlap(Box)
  (params (OverlappedComponent :type Primitive%20Component%20Object%20Reference) (OtherActor :type Actor%20Object%20Reference) (OtherComp :type Primitive%20Component%20Object%20Reference) (OtherBodyIndex :type Integer) (bFromSweep :type Boolean) (SweepResult :type Hit%20Result%20Structure%20%28by%20ref%29))
  ;[1 1 1] NewTileGenereation
  (Utilities|Casting|CastToThirdPersonCharacter OtherActor)
  (bind _asthird_person_game_mode (Utilities|Casting|CastToThirdPersonGameMode (Game|GetGameMode)))
  (Default|SpawnGround _asthird_person_game_mode)
  (Default|SpawnGround _asthird_person_game_mode)
  (Utilities|FlowControl|Delay 2.0)
  (Actor|DestroyActor))

(event EventBeginPlay
  (CallFunction|SpawnObjectAroundMapRight)
  (CallFunction|SpawnObjectAroundMapLeft))

(fn ConstructionScript)

(fn SpawnObjectAroundMapRight
  (bind _objectspawnright (Variables|Default|GetObjectSpawnRight))
  (bind _returnvalue (Transformation|GetWorldTransform _objectspawnright))
  (Game|SpawnActorfromClass "/Game/RunnerFiles/Blueprints/MapBackgroundObjects.MapBackgroundObjects_C" (Math|Transform|MakeTransform (Math|Vector|MakeVector (.x (.location _returnvalue)) (Math|Random|RandomFloatinRange 7e+02 1.25e+03) (.z (.location _returnvalue))) (.rotation _returnvalue) "1,1,1") "Undefined" 0 0))

(fn SpawnObjectAroundMapLeft
  (bind _objectspawnleft (Variables|Default|GetObjectSpawnLeft))
  (bind _returnvalue (Transformation|GetWorldTransform _objectspawnleft))
  (Game|SpawnActorfromClass "/Game/RunnerFiles/Blueprints/MapBackgroundObjects.MapBackgroundObjects_C" (Math|Transform|MakeTransform (Math|Vector|MakeVector (.x (.location _returnvalue)) (Math|Random|RandomFloatinRange -7e+02 -1.25e+03) (.z (.location _returnvalue))) (.rotation _returnvalue) "1,1,1") "Undefined" 0 0))