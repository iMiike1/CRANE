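; Magnet pickup for a runner game that grants the player a timed magnet power-up.
; When a ThirdPersonCharacter overlaps it, it hides its Magnet component and sets MagnetActive on that character.
; After a ten-second delay it calls DeactivateMagnet on player character 0, then destroys itself.
; Debug strings print at each stage, and collision stays enabled while the hidden pickup waits.
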(event EventBeginPlay)

(event Collision|EventActorBeginOverlap
  (params (OtherActor :type Actor%20Object%20Reference))
  (bind _asthird_person_character (Utilities|Casting|CastToThirdPersonCharacter OtherActor))
  (Rendering|SetVisibility (Variables|Default|GetMagnet) false false)
  (Variables|/Game/ThirdPersonBP/Blueprints/ThirdPersonCharacter.ThirdPersonCharacter_C|SetMagnetActive _asthird_person_character true)
  (Development|PrintString "MagnetActive")
  (Utilities|FlowControl|Delay 1e+01)
  (Development|PrintString "magnetinactive")
  (bind _asthird_person_character_2 (Utilities|Casting|CastToThirdPersonCharacter (Game|GetPlayerCharacter 0)))
  (Default|DeactivateMagnet _asthird_person_character_2)
  (Development|PrintString "Deactivated")
  (Actor|DestroyActor))

(event EventTick
  (params (DeltaSeconds :type Float%20%28single-precision%29)))

(fn ConstructionScript)